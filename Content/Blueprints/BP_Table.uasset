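; BP_Table is a table Blueprint that hosts the roll button UI, showing turn count and whether rolling is available.
; On BeginPlay it casts the RollBtn component's widget to WBP_RollBtn and caches the reference.
; UpdateTurn and UpdateRollBtn events forward turn counts and the can-roll state to that widget, which handles the display and active or inactive switching.
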(event `self.ReceiveBeginPlay`
  (bind _aswbp_roll_btn (cast `/Game/Blueprints/WBP/WBP_RollBtn` (`WidgetComponent.GetWidget` (`self.RollBtn`))))
  (set `self.RollBtnUI` _aswbp_roll_btn))

(event `/Game/Blueprints/BPI/BPI_UpdateTable.UpdateTurn`
  (params (Left :type Integer) (Max :type Integer))
  (`/Game/Blueprints/WBP/WBP_RollBtn.UpdateTurnCount` (`self.RollBtnUI`) Left Max))

(event `/Game/Blueprints/BPI/BPI_UpdateTable.UpdateRollBtn`
  (params (bCanRoll :type Boolean))
  (if bCanRoll
    (`/Game/Blueprints/WBP/WBP_RollBtn.ActiveRollBtn` (`self.RollBtnUI`))
    (else
      (`/Game/Blueprints/WBP/WBP_RollBtn.InActiveRollBtn` (`self.RollBtnUI`)))))

(fn `UserConstructionScript`)