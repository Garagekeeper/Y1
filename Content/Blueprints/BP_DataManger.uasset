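; Data manager Blueprint that serves shop items and their effects from the item and effect data tables it sets on BeginPlay.
; GetShopItems gathers items below their MaxStack, shuffles them and returns three picks, incrementing each pick's count in ItemStackMap as it is offered.
; GetItemEffect scans the effect table and returns every row whose ItemID matches the requested one.
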(event `self.ReceiveBeginPlay`
  (`|ExecutionSequence`
    (:`then_0`
      (set `self.ItemData` "/Game/Data/DT_ItemList.DT_ItemList")
      (set `self.ItemEffectData` "/Game/Data/DT_EffectList.DT_EffectList"))))

(fn `GetItemEffect`
  (params (ItemId :type Name))
  (returns (Effects :type "Array of /Game/Data/ST_ItemEffect Structure"))
  (locals (ItemEffects :type "Array of /Game/Data/ST_ItemEffect Structure") (Temp :type "/Game/Data/ST_ItemEffect Structure"))
  (bind _outrownames (`DataTableFunctionLibrary.GetDataTableRowNames` (`self.ItemEffectData`)))
  (for _array_element _outrownames
    (bind _returnvalue (`|GetDataTableRow` (`self.ItemEffectData`) _array_element)
      (:`then`
        (bind _output_get (set `local.Temp` _returnvalue))
        (if (== (`.ItemID_2_F1B6FC434CDE7D4A334B7BAA685DA33D` (break `/Game/Data/ST_ItemEffect` _output_get)) ItemId)
          (`KismetArrayLibrary.Array_Add` (`local.ItemEffects`) (`local.Temp`))))))
  (return (`local.ItemEffects`)))

(fn `GetShopItems`
  (returns (NewParam :type "Array of /Game/Data/ST_ShopItem Structure"))
  (locals (ShopItemStructure :type "/Game/Data/ST_ShopItem Structure") (Candidate :type "Array of Name") (ItemArray :type "Array of /Game/Data/ST_ShopItem Structure") (Temp :type Name))
  (bind _itemstackmap (`self.ItemStackMap`))
  (bind _outrownames (`DataTableFunctionLibrary.GetDataTableRowNames` (`self.ItemData`)))
  (for _array_element _outrownames
    (bind _returnvalue (`|GetDataTableRow` (`self.ItemData`) _array_element)
      (:`then`
        (bind _output_get (set `local.ShopItemStructure` _returnvalue))
        (bind (_value _returnvalue_2) (`BlueprintMapLibrary.Map_Find` (`self.ItemStackMap`) _array_element))
        (if _returnvalue_2
          (if (< _value (`.MaxStack_20_31A7A9B64F3482CE8B240BB85BD58A33` (break `/Game/Data/ST_ShopItem` _output_get)))
            (`KismetArrayLibrary.Array_Add` (`local.Candidate`) _array_element :!label _label))
          (else
            (goto _label))))))
  (`KismetArrayLibrary.Array_Shuffle` (`local.Candidate`))
  (for _index (range 3)
    (set `local.Temp` (`|GetArrayItem` (`local.Candidate`) _index))
    (bind _returnvalue_3 (`|GetDataTableRow` (`self.ItemData`) (`local.Temp`))
      (:`then`
        (`KismetArrayLibrary.Array_Add` (`local.ItemArray`) _returnvalue_3)
        (`BlueprintMapLibrary.Map_Add` _itemstackmap (`local.Temp`) (+ (`BlueprintMapLibrary.Map_Find` _itemstackmap (`local.Temp`)) 1)))))
  (return (`local.ItemArray`)))

(fn `UserConstructionScript`)