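; BP_ScoreBoard is a scoreboard Blueprint that displays scores and multipliers through a widget component.
; On BeginPlay it casts the component's widget to WBP_SocreUI, caches it and registers itself as that widget's parent.
; Its events pass calls straight to the widget to update calculated and fixed scores, update individual and total multipliers, clear undecided scores, or empty the whole board.
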(event `self.ReceiveBeginPlay`
  (bind _aswbp_socre_ui (cast `/Game/Blueprints/WBP/WBP_SocreUI` (`WidgetComponent.GetWidget` (`self.Widget`))))
  (bind _output_get (set `self.ScoreBoardUI` _aswbp_socre_ui))
  (`/Game/Blueprints/WBP/WBP_SocreUI.Setparent` _output_get self))

(event `/Game/Blueprints/BPI/BPI_UpdateSocreBoards.UpdateScoreTexts`
  (params (`Display Scores` :type "/Game/Blueprints/ST_Scores Structure") (`Fixed Score` :type "/Game/Blueprints/ST_Scores Structure"))
  (`/Game/Blueprints/WBP/WBP_SocreUI.UpdateScore` (`self.ScoreBoardUI`) `Display Scores` `Fixed Score`))

(event `/Game/Blueprints/BPI/BPI_UpdateSocreBoards.EraseUnSelected`
  (`/Game/Blueprints/WBP/WBP_SocreUI.SetUndecidedScoreEmpty` (`self.ScoreBoardUI`)))

(event `/Game/Blueprints/BPI/BPI_UpdateSocreBoards.InitScoreboard`
  (`/Game/Blueprints/WBP/WBP_SocreUI.SetAllEmpty` (`self.ScoreBoardUI`)))

(event `/Game/Blueprints/BPI/BPI_UpdateSocreBoards.UpdateMultiplier`
  (params (InMultipliers :type "/Game/Blueprints/ST_Multiplier Structure") (InTotalMultiplier :type Integer))
  (`/Game/Blueprints/WBP/WBP_SocreUI.UpdateMultiplier` (`self.ScoreBoardUI`) InMultipliers InTotalMultiplier))

(fn `UserConstructionScript`)