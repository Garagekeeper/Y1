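; BP_MainHUD is the main HUD Blueprint, managing the on-screen message and result widgets.
; On BeginPlay it adds WBP_HUDMessage to the viewport, and the PrintMsg and DisableMsg events forward to it to show or deactivate messages.
; ShowRes lazily creates WBP_ShowRes and pauses the game, while later calls with a valid widget only invoke its StartRes.
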(event `self.ReceiveBeginPlay`
  (bind _returnvalue (`|CreateWidget` "/Game/Blueprints/WBP/WBP_HUDMessage.WBP_HUDMessage_C"))
  (bind _output_get (set `self.MsgHUD` _returnvalue))
  (`UserWidget.AddToViewport` _output_get 0))

(event `/Game/Blueprints/BPI/BPI_MsgInteract.DisableMsg`
  (`/Game/Blueprints/WBP/WBP_HUDMessage.InActiveMessage` (`self.MsgHUD`)))

(event `/Game/Blueprints/BPI/BPI_MsgInteract.PrintMsg`
  (params (InMsg :type String))
  (`/Game/Blueprints/WBP/WBP_HUDMessage.PrintMessage` (`self.MsgHUD`) InMsg))

(event `/Game/Blueprints/BPI/BPI_StageResShow.ShowRes`
  (`/Engine/EditorBlueprintResources/StandardMacros.IsValid` (`self.ResultUI`)
    (:`Is Valid`
      (`/Game/Blueprints/WBP/WBP_ShowRes.StartRes` (`self.ResultUI`)))
    (:`Is Not Valid`
      (bind _returnvalue (`|CreateWidget` "/Game/Blueprints/WBP/WBP_ShowRes.WBP_ShowRes_C"))
      (bind _output_get (set `self.ResultUI` _returnvalue))
      (`UserWidget.AddToViewport` _output_get 0)
      (`GameplayStatics.SetGamePaused` true))))

(fn `UserConstructionScript`)