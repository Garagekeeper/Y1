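; BP_Chair is an interactable chair that toggles the calling character between sitting and standing.
; On Interact it queries the caller's sit state; to seat it, it disables movement, saves its location, snaps it to the Arrow component's transform and sends SitMessage.
; To stand it up, it restores walking mode and passes the saved location through UnSitMessage.
; The player overlap check leads to no action.
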(event `self.ReceiveActorBeginOverlap`
  (params (OtherActor :type "Actor Object Reference"))
  (if (== OtherActor (`GameplayStatics.GetPlayerPawn` 0))
    _))

(event `/Game/Blueprints/BPI_Interactible.Interact`
  (params (Caller :type "Character Object Reference"))
  (bind _charactermovement (`Character.CharacterMovement` Caller))
  (bind _arrow (`self.Arrow`))
  (bind _bsit (message `/Game/Blueprints/BPI_Sittable.IsSit` Caller))
  (if _bsit
    (`CharacterMovementComponent.SetMovementMode` _charactermovement "MOVE_Walking" 0)
    (message `/Game/Blueprints/BPI_Sittable.UnSit` Caller (`self.BeforeSitLocaion`))
    (else
      (`CharacterMovementComponent.DisableMovement` _charactermovement)
      (set `self.BeforeSitLocaion` (`self.K2_GetActorLocation` Caller))
      (`self.K2_SetActorLocationAndRotation` Caller (`SceneComponent.K2_GetComponentLocation` _arrow) (`SceneComponent.K2_GetComponentRotation` _arrow) false false)
      (message `/Game/Blueprints/BPI_Sittable.Sit` Caller))))

(fn `UserConstructionScript`)