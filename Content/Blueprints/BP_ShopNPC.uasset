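; Shop NPC Blueprint that opens a shop UI offering item effects from the game's data manager.
; Interact creates WBP_Shop, fills it with shop items, enables input and notifies the player pawn, then locks until InitInteract.
; SelectEffect looks up the chosen effect by name, applies it through GM_InGame and closes the shop.
; Refresh refetches items, and leaving DetectArea disables input.
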(event `self.ReceiveBeginPlay`)

(event `/Game/Blueprints/BPI/BPI_Interactible.Interact`
  (params (Caller :type "Character Object Reference"))
  (if (`self.bCanInteract`)
    (bind _returnvalue (`|CreateWidget` "/Game/Blueprints/WBP/WBP_Shop.WBP_Shop_C"))
    (bind _output_get (set `self.ShopUI` _returnvalue))
    (`/Game/Blueprints/WBP/WBP_Shop.SetParent` _output_get self)
    (`UserWidget.AddToViewport` (`self.ShopUI`) 0)
    (bind _output_get_2 (`self.GetItemEffectFromDataTable`))
    (`/Game/Blueprints/WBP/WBP_Shop.InitCard` (`self.ShopUI`) _output_get_2)
    (`self.EnableInput` (`GameplayStatics.GetPlayerController` 0))
    (set `self.bCanInteract` false)
    (message `/Game/Blueprints/BPI/BPI_ShopInterface.OpenShop` (`GameplayStatics.GetPlayerPawn` 0) (`self.ShopUI`))))

(event `/Game/Blueprints/BPI/BPI_Interactible.ExitInteract`
  (`Widget.RemoveFromParent` (`self.ShopUI`))
  (message `/Game/Blueprints/BPI/BPI_ShopInterface.ExitShop` (`GameplayStatics.GetPlayerPawn` 0)))

(event `/Game/Blueprints/BPI/BPI_Interactible.InitInteract`
  (set `self.bCanInteract` true))

(event `SelectEffect`
  (params (InInedex :type Integer))
  (bind _asgm_in_game (cast `/Game/Blueprints/FrameWork/GM_InGame` (`GameplayStatics.GetGameMode`)))
  (bind _effects (`/Game/Blueprints/BP_DataManger.GetItemEffect` (`/Game/Blueprints/FrameWork/GM_InGame.DataManager` _asgm_in_game) (`KismetStringLibrary.Conv_StringToName` (`KismetStringLibrary.Replace` (`KismetTextLibrary.Conv_TextToString` (`.ItemName_2_4DA203B64A5464D94AB075AC40751EF5` (break `/Game/Data/ST_ShopItem` (`|GetArrayItem` (`self.EffectArr`) InInedex)))) " "))))
  (`/Game/Blueprints/FrameWork/GM_InGame.ApplyItmeEffect` _asgm_in_game _effects)
  (`self.ExitInteract`))

(event `Refresh`
  (bind _output_get (`self.GetItemEffectFromDataTable`))
  (`/Game/Blueprints/WBP/WBP_Shop.InitCard` (`self.ShopUI`) _output_get))

(event `self.DetectArea.OnComponentEndOverlap`
  (params (OverlappedComponent :type "PrimitiveComponent Object Reference") (OtherActor :type "Actor Object Reference") (OtherComp :type "PrimitiveComponent Object Reference") (OtherBodyIndex :type Integer))
  (`self.DisableInput` (`GameplayStatics.GetPlayerController` 0)))

(fn `GetItemEffectFromDataTable`
  (returns (Output_Get :type "Array of /Game/Data/ST_ShopItem Structure"))
  (bind _datamanager (`/Game/Blueprints/BPFL/BPFL_Game.GetDataManager`))
  (bind _newparam (`/Game/Blueprints/BP_DataManger.GetShopItems` _datamanager))
  (bind _output_get (set `self.EffectArr` _newparam))
  (return _output_get))

(fn `UserConstructionScript`)