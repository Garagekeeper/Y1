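; Physics-driven clickable dice actor that rolls, reports its upper face and can be toggled as kept through GM_InGame.
; While evaluating, Tick waits for velocities to settle, then picks the face whose local-axis dot product with world up is closest to a target and broadcasts roll completion.
; Timelines move it, with physics off and clicks blocked, to keep, display (rotated by rolled face) or previous positions, each broadcasting on finish.
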(event `self.ReceiveBeginPlay`)

(event `self.ReceiveTick`
  (params (DeltaSeconds :type "Float (single-precision)"))
  (if (`self.bCanEvaluate`)
    (if (and (`KismetMathLibrary.NearlyEqual_FloatFloat` (`KismetMathLibrary.VSize` (`self.GetVelocity`))) (`KismetMathLibrary.NearlyEqual_FloatFloat` (`KismetMathLibrary.VSize` (`PrimitiveComponent.GetPhysicsAngularVelocityInDegrees` (`self.Dice`) "None"))))
      ; Wait until stop completely
      (bind _output_get (set `self.Elapsed` (+ DeltaSeconds (`self.Elapsed`))))
      (if (and (>= _output_get (`self.SettlingTine`)) (not (`self.bAddImpact`)) (`self.bCanEvaluate`))
        (bind _upperface (`self.EvaluateDiveRes`))
        (set `self.UpFaceNumber` _upperface)
        (set `self.bCanEvaluate` false)
        (`self.OnRollDone`)))))

(event `/Game/Blueprints/BPI/BPI_DiceRoll.StartRoll`
  (if (`self.bCanReroll`)
    (set `self.bCanEvaluate` true)
    (set `self.bAddImpact` true)
    (else
      (`KismetSystemLibrary.PrintString` "Something goes wrong, trying to reroll kept(Cna't Reroll)Dice"))))

(event `/Game/Blueprints/BPI/BPI_DiceRoll.ReadyToRoll`
  (`PrimitiveComponent.SetSimulatePhysics` (`self.Dice`) true)
  (set `self.bCanReroll` true))

(event `self.ReceiveHit`
  (params (MyComp :type "PrimitiveComponent Object Reference") (Other :type "Actor Object Reference") (OtherComp :type "PrimitiveComponent Object Reference") (bSelfMoved :type Boolean) (HitLocation :type "Vector Structure") (HitNormal :type "Vector Structure") (NormalImpulse :type "Vector Structure") (Hit :type "HitResult Structure (by ref)"))
  (if (and (`self.bAddImpact`) (`self.bCanEvaluate`) (`self.bCanImpulse`) (`KismetSystemLibrary.DoesImplementInterface` Other "/Game/Blueprints/BPI/BPI_DiceMove.BPI_DiceMove_C"))
    _))

(event `/Game/Blueprints/BPI/BPI_DiceRoll.ThrowDice`
  (set `self.bAddImpact` false)
  (`PrimitiveComponent.SetPhysicsLinearVelocity` (`self.Dice`) (0.0 0.0 0.0) false "None"))

(event `self.Dice.OnClicked`
  (params (TouchedComponent :type "PrimitiveComponent Object Reference") (ButtonPressed :type "Key Structure"))
  (if (`self.bCanInteract`)
    (set `self.bCanReroll` (not (`self.bCanReroll`)))
    (bind _asgm_in_game (cast `/Game/Blueprints/FrameWork/GM_InGame` (`GameplayStatics.GetGameMode`)))
    (`/Game/Blueprints/FrameWork/GM_InGame.DiceKeepToggle` _asgm_in_game self)))

(event `/Game/Blueprints/BPI/BPI_DiceMove.MoveToKeepZone`
  (params (DestPostion :type "Vector Structure"))
  (`/Game/Blueprints/BPI/BPI_DiceInteraction.InActiveClickEvent`)
  (`PrimitiveComponent.SetSimulatePhysics` (`self.Dice`) false)
  (bind _output_get (set `self.StartPos` (`self.K2_GetActorLocation`)))
  (bind (_direction _movealpha) (`Timeline|TL_DiceMove` :!via `PlayFromStart` :!label _label)
    (:`Update`
      (`self.K2_SetActorLocation` (`KismetMathLibrary.VLerp` _output_get DestPostion _movealpha)))
    (:`Finished`
      (`self.OnKeepDone`)
      (`/Game/Blueprints/BPI/BPI_DiceInteraction.ActiveClickEvent`))))

(event `/Game/Blueprints/BPI/BPI_DiceMove.StopAllTimeLine`
  (`|ExecutionSequence`
    (:`then_0`
      (goto _label :!via `Stop`))
    (:`then_1`
      (bind (_direction _movealpha) (`Timeline|Timeline` :!via `Stop` :!label _label_2)
        (:`Update`
          (`self.K2_SetActorLocationAndRotation` (`KismetMathLibrary.VLerp` (`self.K2_GetActorLocation`) (stale `/Game/Blueprints/BPI/BPI_DiceMove.MoveToDisplayZone` DestPos) _movealpha) (`KismetMathLibrary.RLerp` (`self.K2_GetActorRotation`) (select `int` (`self.UpFaceNumber`) :`0` (struct) :`1` (struct :`Roll` 90.0) :`2` (struct) :`3` (struct :`Pitch` 90.0 :`Yaw` 180.0) :`4` (struct :`Pitch` -90.0 :`Yaw` 180.0) :`5` (struct :`Roll` -180.0) :`6` (struct :`Roll` -90.0) :!type "Rotator Structure") _movealpha)))
        (:`Finished`
          (`self.OnDisplayDone`)
          (`/Game/Blueprints/BPI/BPI_DiceInteraction.ActiveClickEvent`))))
    (:`then_2`
      (bind (_direction_2 _movealpha_2) (`Timeline|Timeline_0` :!via `Stop` :!label _label_3)
        (:`Update`
          (`self.K2_SetActorLocation` (`KismetMathLibrary.VLerp` (`self.K2_GetActorLocation`) (`self.StartPos`) _movealpha_2)))
        (:`Finished`
          (`self.OnMoveBeforeDone`)
          (`/Game/Blueprints/BPI/BPI_DiceInteraction.ActiveClickEvent`))))))

(event `/Game/Blueprints/BPI/BPI_DiceMove.MoveToDisplayZone`
  (params (DestPos :type "Vector Structure"))
  (`/Game/Blueprints/BPI/BPI_DiceInteraction.InActiveClickEvent`)
  (`PrimitiveComponent.SetSimulatePhysics` (`self.Dice`) false)
  (goto _label_2 :!via `PlayFromStart`))

(event `/Game/Blueprints/BPI/BPI_DiceMove.MoveToPosBefore`
  (`/Game/Blueprints/BPI/BPI_DiceInteraction.InActiveClickEvent`)
  (`PrimitiveComponent.SetSimulatePhysics` (`self.Dice`) false)
  (goto _label_3 :!via `PlayFromStart`))

(event `/Game/Blueprints/BPI/BPI_DiceInteraction.InActiveClickEvent`
  (set `self.bCanInteract` false))

(event `/Game/Blueprints/BPI/BPI_DiceInteraction.ActiveClickEvent`
  (set `self.bCanInteract` true))

(fn `CanReroll`
  (returns (bCanReroll :type Boolean))
  (return (`self.bCanReroll`)))

(fn `EvaluateDiveRes`
  (returns (UpperFace :type Integer))
  (`self.SetFaceVector`)
  (`self.SetDotRes`)
  (bind _upperface (`self.GetUpperFace`))
  (return _upperface))

(fn `GetUpperFace`
  (returns (UpperFace :type Integer))
  (locals (MinVal :type "Float (double-precision)" :default 1000000.0) (CurrIndex :type Integer) (FaceUpDotRes :type "Float (double-precision)" :default 1.0))
  (for (_array_element _array_index) (`self.DotResArray`)
    (bind _returnvalue (`KismetMathLibrary.Abs` (- _array_element (`local.FaceUpDotRes`))))
    (if (< _returnvalue (`local.MinVal`))
      (set `local.MinVal` _returnvalue)
      (set `local.CurrIndex` _array_index)))
  (return (`local.CurrIndex`)))

(fn `GetUpSideFace`
  (returns (OutFace :type Integer))
  (return (`self.UpFaceNumber`)))

(fn `UserConstructionScript`
  (for _ (range (+ (`self.DiceFaceMax`) 1))
    (`KismetArrayLibrary.Array_Add` (`self.DotResArray`))))