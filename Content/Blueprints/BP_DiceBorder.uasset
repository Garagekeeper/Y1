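; BP_DiceBorder is a dice border that supplies world positions for pocketing and aligning dice.
; On BeginPlay it caches two numbered sets of static mesh socket locations, pocket and align, and sizes an occupancy array.
; GetEmptySocketLocation returns the first free pocket and marks it taken; despite the name DicePocketEmpty, true means occupied.
; GetAllignSocketArray exposes the align positions, and nothing here frees a pocket.
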(event `self.ReceiveBeginPlay`
  (for _index (range (+ (`self.PocketCnt`) 1))
    (`KismetArrayLibrary.Array_Add` (`self.PocketSocketArray`) (`SceneComponent.GetSocketLocation` (`self.StaticMesh`) (`KismetStringLibrary.Conv_StringToName` (`KismetStringLibrary.BuildString_Int` (`self.PocketSocketName`) "" _index))))
    (`KismetArrayLibrary.Array_Add` (`self.AllignSocketArray`) (`SceneComponent.GetSocketLocation` (`self.StaticMesh`) (`KismetStringLibrary.Conv_StringToName` (`KismetStringLibrary.BuildString_Int` "" (`self.AllighSocketName`) _index)))))
  (`KismetSystemLibrary.PrintString` "Hello")
  (`KismetArrayLibrary.Array_Resize` (`self.bDicePocketEmpty`) (`self.PocketCnt`)))

(fn `GetAllignSocketArray`
  (returns (OutArray :type "Array of Vector Structure"))
  (return (`self.AllignSocketArray`)))

(fn `GetEmptySocketLocation`
  (returns (`Out Socet Locaion` :type "Vector Structure"))
  (locals (Res :type "Vector Structure"))
  (for (_array_element _array_index) (`self.PocketSocketArray`)
    (if (== (`|GetArrayItem` (`self.bDicePocketEmpty`) _array_index) false)
      (set `local.Res` _array_element)
      (`KismetArrayLibrary.Array_Set` (`self.bDicePocketEmpty`) _array_index true)
      (break)))
  (return (`local.Res`)))

(fn `UserConstructionScript`)