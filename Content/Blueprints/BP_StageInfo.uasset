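; BP_StageInfo is a Blueprint that displays stage information, namely the current score and a remaining value, through a widget component.
; On BeginPlay it casts the component's widget to WBP_StageInfo, caches it and passes itself to the widget as parent.
; The UpdateCurrentScore and UpdateRemain events forward incoming values straight to the cached widget's update functions.
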(event `self.ReceiveBeginPlay`
  (bind _aswbp_stage_info (cast `/Game/Blueprints/WBP_StageInfo` (`WidgetComponent.GetWidget` (`self.Widget`))))
  (set `self.StageInfoUI` _aswbp_stage_info)
  (`/Game/Blueprints/WBP_StageInfo.Setparent` _aswbp_stage_info self))

(event `/Game/Blueprints/BPI_StageInfoUpdate.UpdateCurrentScore`
  (params (CurrentScore :type Integer))
  (`/Game/Blueprints/WBP_StageInfo.UpdateCurrScores` (`self.StageInfoUI`) CurrentScore))

(event `/Game/Blueprints/BPI_StageInfoUpdate.UpdateRemain`
  (params (InRemain :type Integer))
  (`/Game/Blueprints/WBP_StageInfo.UpdateCurrentRemain` (`self.StageInfoUI`) InRemain))

(fn `UserConstructionScript`)