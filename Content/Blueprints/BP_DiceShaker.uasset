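; Dice cup actor that the player clicks to shake and releases to throw, relaying both inputs to GM_InGame.
; One timeline jitters the cup; another moves and rolls it while pushing a bound volume like a piston.
; An event on the throw timeline drops detector and wall collision and asks the game mode for an up-vector impulse; collision returns on finish.
; Also returns mesh socket locations as dice positions.
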(event `self.ReceiveBeginPlay`
  (set `self.StartPos` (`self.K2_GetActorLocation`)))

(event `ShakeShaker`
  (bind (_currentlocation_x _currentlocation_y _currentlocation_z) (`KismetMathLibrary.BreakVector` (`self.CurrentLocation`)))
  (set `self.CurrentLocation` (`self.K2_GetActorLocation`))
  (bind (_direction _xalpha _newtrack_2) (`Timeline|TL_Shaker` :!label _label)
    (:`Update`
      (`self.K2_SetActorLocation` (`KismetMathLibrary.MakeVector` (+ (* _xalpha 2.0) _currentlocation_x) (+ (* _xalpha 2.0) _currentlocation_y) (+ _newtrack_2 _currentlocation_z)) true))))

(event `Stop Shaker`
  (goto _label :!via `Stop`))

(event `RotateShaker`
  (bind (_startpistonvec_x _startpistonvec_y _startpistonvec_z) (`KismetMathLibrary.BreakVector` (`self.StartPistonvec`)))
  (bind (_startpos_x _startpos_y _startpos_z) (`KismetMathLibrary.BreakVector` (`self.StartPos`)))
  (set `self.StartPos` (`self.K2_GetActorLocation`))
  (set `self.StartPistonvec` (`SceneComponent.RelativeLocation` (`self.CupBoundVolume8`)))
  (bind (_direction _ymove _rotate _zmove _pistone) (`Timeline|TL_ThrowDIce` :!via `PlayFromStart`)
    (:`Update`
      (`self.K2_SetActorLocationAndRotation` (`KismetMathLibrary.MakeVector` _startpos_x (+ (* _ymove (`self.moveWidth`)) _startpos_y) (+ _startpos_z (* _zmove 10.0))) (`KismetMathLibrary.MakeRotator` _rotate))
      (`SceneComponent.K2_SetRelativeLocation` (`self.CupBoundVolume8`) (`KismetMathLibrary.MakeVector` _startpistonvec_x _startpistonvec_y (+ _startpistonvec_z (* _pistone 150.0))) false false))
    (:`Finished`
      (`PrimitiveComponent.SetCollisionEnabled` (`self.DiceCollsionDetector`) "QueryAndPhysics")
      (`PrimitiveComponent.SetCollisionEnabled` (`self.CupBoundVolume5`) "PhysicsOnly")
      (`PrimitiveComponent.SetCollisionEnabled` (`self.CupBoundVolume7`) "PhysicsOnly"))
    (:`Event`
      (`PrimitiveComponent.SetCollisionEnabled` (`self.DiceCollsionDetector`) "NoCollision")
      (message `/Game/Blueprints/BPI_ImpulseAddable.AddImpulseToActor` (`GameplayStatics.GetGameMode`) (`SceneComponent.GetUpVector` (`self.DiceShakerMesh`)))
      (`PrimitiveComponent.SetCollisionEnabled` (`self.CupBoundVolume5`) "NoCollision")
      (`PrimitiveComponent.SetCollisionEnabled` (`self.CupBoundVolume7`) "NoCollision"))))

(event `Throw`
  (set `self.bPressed` false))

(event `self.DiceCollsionDetector.OnClicked`
  (params (TouchedComponent :type "PrimitiveComponent Object Reference") (ButtonPressed :type "Key Structure"))
  (bind _asgm_in_game (cast `/Game/Blueprints/FrameWork/GM_InGame` (`GameplayStatics.GetGameMode`)))
  (`/Game/Blueprints/FrameWork/GM_InGame.StartShake` _asgm_in_game))

(event `self.DiceCollsionDetector.OnReleased`
  (params (TouchedComponent :type "PrimitiveComponent Object Reference") (ButtonReleased :type "Key Structure"))
  (bind _asgm_in_game (cast `/Game/Blueprints/FrameWork/GM_InGame` (`GameplayStatics.GetGameMode`)))
  (`/Game/Blueprints/FrameWork/GM_InGame.ThrowDices` _asgm_in_game))

(fn `GetDiceLocationSocket`
  (returns (OutSocketLocationArray :type "Array of Vector Structure"))
  (locals (SocketLocationArray :type "Array of Vector Structure"))
  (for _array_element (`SceneComponent.GetAllSocketNames` (`self.DiceShakerMesh`))
    (`KismetArrayLibrary.Array_Add` (`local.SocketLocationArray`) (`SceneComponent.GetSocketLocation` (`self.DiceShakerMesh`) _array_element)))
  (return (`local.SocketLocationArray`)))

(fn `UserConstructionScript`)